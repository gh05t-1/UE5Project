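; AI controller for enemy pawns that sets up spline-based patrolling, with the patrol behavior itself still unimplemented.
; On possess it stores the pawn, requests its patrol path through a message call, caches the spline point count and resets the current point index.
; The Patrol event only prints a placeholder string, and the GetPatrolPath function is an empty stub.
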(event EventPossess
  (params (PossessedPawn :type Pawn%20Object%20Reference))
  (bind _output_get (Variables|Default|SetEnemy PossessedPawn))
  (bind _patrolpath (Class|EnemyINT|GetPatrolPath(Message) _output_get))
  (bind _output_get_2 (Variables|Default|SetPatrol%20Path _patrolpath))
  (Variables|Default|SetTotal%20Patrol%20Points (Spline|GetNumberOfSplinePoints (Variables|/Game/Blueprints/EnemyAI/PatrolPath_BP.PatrolPath_BP_C|GetSpline _output_get_2)))
  (Variables|Default|SetCurrent%20patrol%20points 0))

(event EventPatrol
  (Development|PrintString "Implement Patrol"))

(fn ConstructionScript)

(fn GetPatrolPath
  (return 0))